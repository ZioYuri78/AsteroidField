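; BP_Asteroid is a physics-driven asteroid actor that is set tumbling with a random spin when play begins.
; BeginPlay assigns the configured mesh, applies the mass override and adds a one-time torque randomized per axis between configurable bounds.
; When Debug is on, Tick draws a sphere around the asteroid and a line to the FlyingPawn player's camera.
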(event EventBeginPlay
  (bind _mintorque (Variables|Rotation|GetMinTorque))
  (bind _maxtorque (Variables|Rotation|GetMaxTorque))
  (Components|StaticMesh|SetStaticMesh (Variables|Default|GetStaticMesh) (Variables|Mesh|GetAsteroidMesh))
  (Class|PrimitiveComponent|SetMassOverrideinKg (Variables|Default|GetStaticMesh) "None" (Variables|Mesh|GetMassInKg) (Variables|Mesh|GetOverrideMass))
  (Class|PrimitiveComponent|AddTorque (Variables|Default|GetStaticMesh) (Math|Vector|MakeVector (Math|Random|RandomFloatinRange _mintorque _maxtorque) (Math|Random|RandomFloatinRange _mintorque _maxtorque) (Math|Random|RandomFloatinRange _mintorque _maxtorque)) "None" (Variables|Rotation|GetAccelChange)))

(event EventTick
  (params (DeltaSeconds :type Float%20%28single-precision%29))
  (bind _returnvalue (Transformation|GetActorLocation))
  ;[1 1 1] Debug
  (if (Variables|Debug|GetDebug)
    (Rendering|Debug|DrawDebugSphere _returnvalue 2.5e+02 12 "(R=0.000000,G=0.318960,B=1.000000,A=1.000000)" 0.0)
    (Rendering|Debug|DrawDebugLine _returnvalue (Transformation|GetWorldLocation (Variables|/Game/FlyingBP/Blueprints/FlyingPawn.FlyingPawn_C|GetCamera (.AsFlying%20Pawn (Utilities|Casting|CastToFlyingPawn (Game|Player|GetPlayerPawn 0))))) "(R=0.000000,G=0.318960,B=1.000000,A=1.000000)" 0.0 0.0)))

(fn ConstructionScript)