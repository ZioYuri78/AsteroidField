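; Asteroid field actor that fills a jittered grid with randomly rotated, scaled HISM instances at construction.
; On the FlyingPawn's camera-transform event, it swaps instances within range and the FOV cone for BP_Asteroid actors, unless a trace hits the player pawn.
; Actors leaving the cone or range revert to instances at their current transform, limiting full actors to what is near and in view.
; Optional debug HUD and traces visualize the swapping.
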(event Custom|UpdateCameraPosition
  (params (Transform :type Transform) (FOV :type Float%20%28single-precision%29))
  (CallFunction|SwapAsteroids Transform FOV (Variables|Swap|GetSwapRange)))

(event EventBeginPlay
  (if (Variables|Debug|GetShowDebugHUD)
    (bind _returnvalue (UserInterface|CreateWidget "/Game/UI/WB_DebugHUD.WB_DebugHUD_C"))
    (UserInterface|Viewport|AddtoViewport _returnvalue 0))
  (bind _asflying_pawn (Utilities|Casting|CastToFlyingPawn (Game|Player|GetPlayerPawn 0)))
  (EventDispatchers|BindEventtoPlayerCameraTransform _asflying_pawn (delegate Custom|UpdateCameraPosition)))

(event EventTick
  (params (DeltaSeconds :type Float%20%28single-precision%29))
  (Variables|Debug|SetInstancedStaticMeshes (Components|InstancedStaticMesh|GetInstanceCount (Variables|Default|GetHierarchicalInstancedStaticMesh)))
  (Variables|Debug|SetBlueprintAsteroids (Utilities|Array|Length (Variables|Default|GetBPInstances))))

(fn ConstructionScript
  (Utilities|IsValid (Variables|Asteroid|GetAsteroidMesh)
    (:Is%20Valid
      (Components|InstancedStaticMesh|ClearInstances (Variables|Default|GetHierarchicalInstancedStaticMesh))
      (Utilities|FlowControl|Sequence
        (:then_0
          (Components|StaticMesh|SetStaticMesh (Variables|Default|GetHierarchicalInstancedStaticMesh) (Variables|Asteroid|GetAsteroidMesh)))
        (:then_1
          (Components|InstancedStaticMesh|SetCullDistances (Variables|Default|GetHierarchicalInstancedStaticMesh) (Variables|Performance|GetStartCullDistance) (Variables|Performance|GetEndCullDistance)))
        (:then_2
          (CallFunction|CreateAsteroidField))))))

(fn SwapAsteroids
  (params (CameraTransform :type Transform) (ViewAngle :type Float%20%28single-precision%29) (Range :type Float%20%28single-precision%29))
  (bind (_location _rotation) (Math|Transform|BreakTransform CameraTransform))
  (bind _returnvalue (/ ViewAngle 2.0))
  (bind _bpinstances (Variables|Default|GetBPInstances))
  (bind _hierarchicalinstancedstaticmesh (Variables|Default|GetHierarchicalInstancedStaticMesh))
  (bind _offsetfov (Variables|Swap|GetOffsetFOV))
  (bind _returnvalue_2 (Math|Vector|GetForwardVector _rotation))
  (bind _returnvalue_3 (Class|InstancedStaticMeshComponent|GetInstancesOverlappingSphere _hierarchicalinstancedstaticmesh _location Range true))
  (bind _returnvalue_4 (+ _returnvalue _offsetfov))
  ;[1 1 1] Check if we have some instances in range
  (if (> (Utilities|Array|Length _returnvalue_3) 0)
    (for _array_element _returnvalue_3
      ;[1 1 1] For each instances that are in a "view" cone we remove and replace it with a Asteroid Blueprint
      (if (Math|Float|InRange(Float) (Class|KismetMathLibrary|DegAcos (Math|Vector|DotProduct (Math|Vector|Normalize (- (.Location (Math|Transform|BreakTransform (.OutInstanceTransform (Components|InstancedStaticMesh|GetInstanceTransform (Variables|Default|GetHierarchicalInstancedStaticMesh) _array_element true)))) _location)) (Math|Vector|Normalize _returnvalue_2))) 0.0 _returnvalue_4)
        (bind _outhit (Collision|LineTraceByChannel _location (.Location (Math|Transform|BreakTransform (.OutInstanceTransform (Components|InstancedStaticMesh|GetInstanceTransform (Variables|Default|GetHierarchicalInstancedStaticMesh) _array_element true)))) "TraceTypeQuery1" true 0 (select (Variables|Debug|GetShowDebugTraces) "ForOneFrame" "None")))
        (if (!= (.HitActor (Collision|BreakHitResult _outhit)) (Game|Player|GetPlayerPawn 0))
          (bind _returnvalue_5 (Game|SpawnActorfromClass "/Game/Blueprints/BP_Asteroid.BP_Asteroid_C" (.OutInstanceTransform (Components|InstancedStaticMesh|GetInstanceTransform (Variables|Default|GetHierarchicalInstancedStaticMesh) _array_element true)) "Undefined" 0 (Variables|Debug|GetShowDebugTraces) (Variables|Asteroid|GetAccelChange) (Variables|Asteroid|GetMinRotationTorque) (Variables|Asteroid|GetMaxRotationTorque) (Variables|Asteroid|GetAsteroidMesh) (Variables|Asteroid|GetOverrideMass) (Variables|Asteroid|GetMassInKg)))
          (Utilities|Array|AddUnique (Variables|Default|GetBPInstances) _returnvalue_5)
          (Class|InstancedStaticMeshComponent|RemoveInstance (Variables|Default|GetHierarchicalInstancedStaticMesh) _array_element))
        (else
          ;[1 1 1] Debug
          (if (Variables|Debug|GetShowDebugTraces)
            (Rendering|Debug|DrawDebugSphere (.Location (Math|Transform|BreakTransform (.OutInstanceTransform (Components|InstancedStaticMesh|GetInstanceTransform (Variables|Default|GetHierarchicalInstancedStaticMesh) _array_element true)))) 2.5e+02 12 "(R=1.000000,G=0.012904,B=0.000000,A=1.000000)" 0.0)
            (Rendering|Debug|DrawDebugLine (.Location (Math|Transform|BreakTransform (.OutInstanceTransform (Components|InstancedStaticMesh|GetInstanceTransform (Variables|Default|GetHierarchicalInstancedStaticMesh) _array_element true)))) _location "(R=1.000000,G=0.012904,B=0.000000,A=1.000000)" 0.0 0.0)
            (Rendering|Debug|DrawDebugSphere _location (Variables|Swap|GetSwapRange) 12 "(R=0.237932,G=0.000000,B=0.370000,A=1.000000)" 0.0))))))
  ;[1 1 1] We pass through spawned Asteroid Blueprint and if are no longer in "view" cone we remove and replace it with a HISM instance
  (if (> (Utilities|Array|Length _bpinstances) 0)
    (for _array_element_2 _bpinstances
      (if (Math|Float|InRange(Float) (Class|KismetMathLibrary|DegAcos (Math|Vector|DotProduct (Math|Vector|Normalize (- (Transformation|GetActorLocation _array_element_2) _location)) (Math|Vector|Normalize _returnvalue_2))) (+ _returnvalue_4 1.0) 1.8e+02)
        (Class|InstancedStaticMeshComponent|AddInstanceWorldSpace (Variables|Default|GetHierarchicalInstancedStaticMesh) (Transformation|GetWorldTransform (Variables|/Game/Blueprints/BP_Asteroid.BP_Asteroid_C|GetStaticMesh _array_element_2)) :!label _label)
        (Actor|DestroyActor _array_element_2)
        (Utilities|Array|RemoveItem (Variables|Default|GetBPInstances) _array_element_2)
        (elif (>= (Math|Vector|VectorLength (- (Transformation|GetActorLocation _array_element_2) _location)) (Variables|Swap|GetSwapRange))
          (goto _label))))))

(fn CreateAsteroidField
  (bind _offsetz (Variables|AsteroidPositionSetup|GetOffsetZ))
  (bind _maxinstancesx (Variables|Instances|GetMaxInstancesX))
  (bind _maxinstancesy (Variables|Instances|GetMaxInstancesY))
  (bind _minasteroidscale (Variables|Asteroid|GetMinAsteroidScale))
  (bind _maxasteroidscale (Variables|Asteroid|GetMaxAsteroidScale))
  (bind _returnvalue (/ _maxinstancesx 2))
  (bind _returnvalue_2 (Math|Random|RandomFloatinRange _minasteroidscale _maxasteroidscale))
  (bind _returnvalue_3 (/ _maxinstancesy 2))
  (for _index (range (* _returnvalue -1) _returnvalue)
    (for _index_2 (range (* _returnvalue_3 -1) _returnvalue_3)
      (Components|InstancedStaticMesh|AddInstance (Variables|Default|GetHierarchicalInstancedStaticMesh) (Math|Transform|MakeTransform (Math|Vector|MakeVector (+ (* _index (Variables|AsteroidPositionSetup|GetOffsetX)) (Math|Random|RandomFloatinRange 0.0 (Variables|AsteroidPositionSetup|GetOffsetDeviationX))) (+ (* _index_2 (Variables|AsteroidPositionSetup|GetOffsetY)) (Math|Random|RandomFloatinRange 0.0 (Variables|AsteroidPositionSetup|GetOffsetDeviationY))) (Math|Random|RandomFloatinRange (* _offsetz -1.0) _offsetz)) (Math|Rotator|MakeRotator (Math|Random|RandomFloatinRange 0.0 3.6e+02) (Math|Random|RandomFloatinRange 0.0 3.6e+02) (Math|Random|RandomFloatinRange 0.0 3.6e+02)) (Math|Vector|MakeVector _returnvalue_2 _returnvalue_2 _returnvalue_2))))))