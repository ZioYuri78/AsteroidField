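; BP_Planet is a planet actor that orbits a referenced Sun around the world Z axis and is lit from its direction.
; The construction script creates a dynamic planet-shader material, passing in rotation speed, cloud speed and initial light direction.
; Each Tick offsets the actor along the orbit, by an angle scaled by delta time squared, and updates the shader's light direction toward the Sun.
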(event EventTick
  (params (DeltaSeconds :type Float%20%28single-precision%29))
  (bind _sun (Variables|Default|GetSun))
  (Utilities|IsValid _sun
    (:Is%20Valid
      (bind _output_get (Variables|Default|SetOrbitDirection (- (Transformation|GetActorLocation) (Transformation|GetActorLocation _sun))))
      (Transformation|AddActorWorldOffset (- (Math|Vector|RotateVectorAroundAxis _output_get (* (Utilities|Time|GetWorldDeltaSeconds) (* DeltaSeconds 36.0)) "0, 0,1.000000") (Variables|Default|GetOrbitDirection)))
      (Rendering|Material|SetVectorParameterValue (Variables|Default|GetMaterialInstance) "Light Direction" (Math|Conversions|ToLinearColor(Vector) (Math|Vector|GetForwardVector (Math|Rotator|FindLookatRotation (Transformation|GetActorLocation) (Transformation|GetActorLocation (Variables|Default|GetSun))))) :!class /Script/Engine.MaterialInstanceDynamic))))

(fn ConstructionScript
  (bind _sun (Variables|Default|GetSun))
  (bind _returnvalue (Rendering|Material|CreateDynamicMaterialInstance (Variables|Default|GetStaticMesh) 0 "/Game/Materials/M_PlanetShader_Inst.M_PlanetShader_Inst" :!class /Script/Engine.PrimitiveComponent))
  (Variables|Default|SetMaterialInstance _returnvalue)
  (Rendering|Material|SetVectorParameterValue _returnvalue "Rotation Speed" (Math|Conversions|ToLinearColor(Vector) (Variables|Default|GetRotationSpeed)) :!class /Script/Engine.MaterialInstanceDynamic)
  (Rendering|Material|SetVectorParameterValue _returnvalue "Clouds Speed" (Math|Conversions|ToLinearColor(Vector) (Variables|Default|GetCloudsSpeed)) :!class /Script/Engine.MaterialInstanceDynamic)
  (Utilities|IsValid _sun
    (:Is%20Valid
      (Rendering|Material|SetVectorParameterValue _returnvalue "Light Direction" (Math|Conversions|ToLinearColor(Vector) (Math|Vector|GetForwardVector (Math|Rotator|FindLookatRotation (Transformation|GetActorLocation) (Transformation|GetActorLocation _sun)))) :!class /Script/Engine.MaterialInstanceDynamic))))