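; BP_Sun is a sun actor that pairs a mesh with a light driven by a shared temperature setting.
; Its construction script applies the temperature to the light, then creates a dynamic material instance on the mesh and passes the light's temperature into its "Max Temperature" parameter.
; If a target actor is set, the script rotates the light to face it, using the light's relative rotation.
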(fn ConstructionScript
  (bind _actor (Variables|Default|GetActor))
  (Class|LightComponent|SetTemperature (Variables|Default|GetSunLight) (Variables|Default|GetSunTemperature))
  (bind _returnvalue (Rendering|Material|CreateDynamicMaterialInstance (Variables|Default|GetSunMesh) 0 0 :!class /Script/Engine.PrimitiveComponent))
  (Variables|Default|SetM_SunInst _returnvalue)
  (Rendering|Material|SetScalarParameterValue (Variables|Default|GetM_SunInst) "Max Temperature" (Variables|/Script/Engine.LightComponent|GetTemperature (Variables|Default|GetSunLight)) :!class /Script/Engine.MaterialInstanceDynamic)
  (Utilities|IsValid _actor
    (:Is%20Valid
      (Transformation|SetRelativeRotation (Variables|Default|GetSunLight) (Math|Rotator|FindLookatRotation (Transformation|GetActorLocation) (Transformation|GetActorLocation _actor)) false false))))